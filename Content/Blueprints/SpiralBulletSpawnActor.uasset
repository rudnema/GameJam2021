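; Actor that fires a spiral stream of Bullet actors from its own location once play begins.
; A delayed loop in the Spiral event spawns a bullet every short interval, up to a thousand times, with yaw derived from the growing counter so each shot rotates further.
; BeginPlay starts the loop and prints a debug string.
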(event `self.ReceiveBeginPlay`
  (`self.Spiral`)
  (`KismetSystemLibrary.PrintString` "XD"))

(event `Spiral`
  (bind _spawncounter (`self.SpawnCounter`))
  (set `self.SpawnCounter` 0.0)
  (if (not (== _spawncounter 1000.0)) :!label _label
    (set `self.SpawnCounter` (+ _spawncounter 1.0))
    (`|SpawnActorFromClass` "/Game/Blueprints/Bullet.Bullet_C" (`KismetMathLibrary.MakeTransform` (`self.K2_GetActorLocation`) (`KismetMathLibrary.MakeRotator` 0.0 0.0 (* (`self.SpawnCounter`) 7.0))) "Undefined" "OverrideRootScale" null null)
    (`KismetSystemLibrary.Delay` 0.05)
    (goto _label)))

(event `self.ReceiveTick`
  (params (DeltaSeconds :type "Float (single-precision)")))

(fn `UserConstructionScript`)