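; Player ship for a 2D meteorite shooter on the XZ plane, destroyed on contact with a meteorite.
; Each tick it rotates toward the mouse cursor, drifts with interpolated input movement and wraps to the opposite side at the play-area limits.
; Firing launches projectiles with a DoOnce/Delay cooldown.
; A flashing timeline keeps collision off after spawn; destruction spawns an explosion and asks the GameMode to respawn the player.
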(event `self.ReceiveTick`
  (params (DeltaSeconds :type "Float (single-precision)"))
  (bind (_returnvalue_x _returnvalue_y _returnvalue_z) (`KismetMathLibrary.BreakVector` (`self.K2_GetActorLocation`)))
  (bind (_returnvalue_x_2 _returnvalue_y_2 _returnvalue_z_2) (`KismetMathLibrary.BreakVector` (`self.K2_GetActorLocation`)))
  (bind (_returnvalue_x_3 _returnvalue_y_3) (`KismetMathLibrary.BreakVector` (`self.K2_GetActorLocation`)))
  (bind _hitresult (`PlayerController.GetHitResultUnderCursorByChannel` (`GameplayStatics.GetPlayerController` 0) "TraceTypeQuery1" true))
  (bind _returnvalue (`KismetMathLibrary.MakeVector` (`self.GetInputAxisValue`) 0.0 (`self.GetInputAxisValue`)))
  (bind _returnvalue_2 (`KismetMathLibrary.Normal` (- (`KismetMathLibrary.MakeVector` (.x (`.Location` (`GameplayStatics.BreakHitResult` _hitresult))) 0.0 (.z (`.Location` (`GameplayStatics.BreakHitResult` _hitresult)))) (`self.K2_GetActorLocation`))))
  (bind _returnvalue_3 (> (`KismetMathLibrary.VSize` _returnvalue) 0.0))
  (if (`GameplayStatics.BreakHitResult` _hitresult)
    _
    (else
      _))
  (`self.K2_SetActorRotation` (`KismetMathLibrary.MakeRotator` 0.0 (* (`KismetMathLibrary.DegAcos` (`KismetMathLibrary.Dot_VectorVector` _returnvalue_2 (0.0 0.0 1.0))) (`KismetMathLibrary.SignOfFloat` (`KismetMathLibrary.Dot_VectorVector` _returnvalue_2 (-1.0 0.0 0.0))))))
  (bind _output_get (set `self.MotionVectorTemp` (`KismetMathLibrary.VInterpTo` (`self.MotionVectorTemp`) (select `bool` _returnvalue_3 :`false` (0.0 0.0 0.0) :`true` (* (`KismetMathLibrary.Normal` _returnvalue) (* (`self.Speed`) (`GameplayStatics.GetWorldDeltaSeconds`)))) (`GameplayStatics.GetWorldDeltaSeconds`) (select `bool` _returnvalue_3 :`false` 1.0 :`true` 5.0 :!type "Float (single-precision)"))))
  (`self.K2_AddActorWorldOffset` _output_get)
  (`|ExecutionSequence`
    (:`then_0`
      (if (> (`KismetMathLibrary.Abs` _returnvalue_x) (`self.X_max`))
        (`self.K2_SetActorLocation` (`KismetMathLibrary.MakeVector` (* (* (`KismetMathLibrary.SignOfFloat` _returnvalue_x) -1.0) (- (`self.X_max`) 20.0)) _returnvalue_y_2 _returnvalue_z_2))))
    (:`then_1`
      (if (> (`KismetMathLibrary.Abs` _returnvalue_z) (`self.Z_Max`))
        (`self.K2_SetActorLocation` (`KismetMathLibrary.MakeVector` _returnvalue_x_3 _returnvalue_y_3 (* (`KismetMathLibrary.SignOfFloat` _returnvalue_z) (- (`self.Z_Max`) 20.0) -1.0)))))))

(event `InputAction|FireAction`
  (params (Key :type "Key Structure"))
  (:`Pressed`
    (`/Engine/EditorBlueprintResources/StandardMacros.DoOnce` false :!label _label
      (:`Completed`
        (bind _returnvalue (`|SpawnActorFromClass` "/Game/Blueprints/BP_ShipProjectileActor.BP_ShipProjectileActor_C" (`KismetMathLibrary.MakeTransform` (`self.K2_GetActorLocation`) (`self.K2_GetActorRotation`)) "AlwaysSpawn" "OverrideRootScale" null null))
        (`ProjectileMovementComponent.SetVelocityInLocalSpace` _returnvalue (0.0 0.0 900.0))
        (`KismetSystemLibrary.Delay` 0.25)
        (goto _label :!via `Reset`)))))

(event `self.playerShip3_blue_Sprite.OnComponentBeginOverlap`
  (params (OverlappedComponent :type "PrimitiveComponent Object Reference") (OtherActor :type "Actor Object Reference") (OtherComp :type "PrimitiveComponent Object Reference") (OtherBodyIndex :type Integer) (bFromSweep :type Boolean) (SweepResult :type "HitResult Structure (by ref)"))
  (cast `/Game/Blueprints/BP_MeteoritActor` OtherActor)
  (`self.K2_DestroyActor`))

(event `self.ReceiveBeginPlay`
  (`PrimitiveComponent.SetCollisionEnabled` (`self.playerShip3_blue_Sprite`) "NoCollision")
  (add `self.OnDestroyed` (delegate `OnDestroyed_Event`))
  (`self.EnableInput` (`GameplayStatics.GetPlayerController` 0))
  (bind (_direction _newtrack_0) (`Timeline|FlashingTimeline`)
    (:`Update`
      (`PaperSpriteComponent.SetSpriteColor` (`self.playerShip3_blue_Sprite`) (make `LinearColor` 1.0 1.0 1.0 _newtrack_0)))
    (:`Finished`
      (`PrimitiveComponent.SetCollisionEnabled` (`self.playerShip3_blue_Sprite`) "QueryAndPhysics"))))

(event `OnDestroyed_Event` :!signature `self.OnDestroyed`
  (params (DestroyedActor :type "Actor Object Reference"))
  (message `/Game/Blueprints/BP_Actions_Interface.TryToSpawnPlayer` (`GameplayStatics.GetGameMode`))
  (`|SpawnActorFromClass` "/Game/Blueprints/BP_ExplosionActor.BP_ExplosionActor_C" (`KismetMathLibrary.Conv_VectorToTransform` (`self.K2_GetActorLocation`)) "AdjustIfPossibleButDontSpawnIfColliding" "OverrideRootScale" null null))

(fn `UserConstructionScript`)