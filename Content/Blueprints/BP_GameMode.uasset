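; Game mode for an Asteroids-style ship game that runs meteorite waves, lives, score and the saved best score.
; A looping timer, its interval randomized once at BeginPlay, spawns 3-5 meteorites at random preset angles by rotating an offset vector around Y.
; Score and life events update the WG_GameHUD widget, respawning the ship or triggering game over.
; BP_SaveGame is loaded or created at start and rewritten at game over when the best is matched or beaten.
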(event `self.ReceiveBeginPlay`
  (set `self.Lives` 3)
  (set `self.Score` 0)
  (set `self.SpawnAngles` (`|MakeArray` 0.0 60.0 120.0 180.0 240.0 300.0 :!type "Float (single-precision)"))
  (`self.SpawnMeteorit`)
  (`KismetSystemLibrary.K2_SetTimer` self "SpawnMeteorit" (`KismetMathLibrary.RandomFloatInRange` 6.0 10.0) true)
  (bind _returnvalue (`|CreateWidget` "/Game/Blueprints/WG_GameHUD.WG_GameHUD_C"))
  (bind _output_get (set `self.HUD_Ref` _returnvalue))
  (`UserWidget.AddToViewport` _output_get 0)
  (`self.CheckSaveGameSlot`))

(event `SpawnMeteorit`
  (bind _spawnpoints_temp (`self.SpawnPoints_Temp`))
  (set `self.SpawnPoints_Temp` (`self.SpawnAngles`))
  (for _ (range (+ (`KismetMathLibrary.RandomIntegerInRange` 3 5) 1))
    (`KismetArrayLibrary.Array_Shuffle` _spawnpoints_temp)
    (bind _returnvalue (`|SpawnActorFromClass` "/Game/Blueprints/BP_MeteoritActor.BP_MeteoritActor_C" (`KismetMathLibrary.MakeTransform` (`KismetMathLibrary.RotateAngleAxis` (`KismetMathLibrary.MakeVector` (`self.X_max`) 0.0 (`self.Z_Max`)) (`|GetArrayItem` _spawnpoints_temp (`KismetMathLibrary.RandomInteger` (`KismetArrayLibrary.Array_Length` _spawnpoints_temp))) (0.0 1.0 0.0))) "AdjustIfPossibleButDontSpawnIfColliding" "OverrideRootScale" null null))
    (set `/Game/Blueprints/BP_MeteoritActor.Type` "NewEnumerator0" _returnvalue)
    (`/Game/Blueprints/BP_MeteoritActor.SetMeteorit` _returnvalue "NewEnumerator0")))

(event `/Game/Blueprints/BP_Actions_Interface.UpdateScore`
  (params (Bonus :type Integer))
  (bind _output_get (set `self.Score` (+ Bonus (`self.Score`))))
  (`TextBlock.SetText` (`/Game/Blueprints/WG_GameHUD.ScoreText` (`self.HUD_Ref`)) (`KismetTextLibrary.Conv_IntToText` _output_get false false)))

(event `/Game/Blueprints/BP_Actions_Interface.TryToSpawnPlayer`
  (bind _savegameinstance_ref (`self.SaveGameInstance_Ref`))
  (`KismetSystemLibrary.Delay` 1.0)
  (bind _output_get (set `self.Lives` (- (`self.Lives`) 1)))
  (`/Game/Blueprints/WG_GameHUD.UpdateLives` (`self.HUD_Ref`) _output_get)
  (`/Engine/EditorBlueprintResources/StandardMacros.CompareInt` (`self.Lives`)
    (:`>`
      (`|SpawnActorFromClass` "/Game/Blueprints/BP_ShipActor.BP_ShipActor_C" (`KismetMathLibrary.MakeTransform` (0.0 0.0 0.0)) "AdjustIfPossibleButDontSpawnIfColliding" "OverrideRootScale" null null))
    (:`==`
      (`/Game/Blueprints/WG_GameHUD.GameOverEvent` (`self.HUD_Ref`))
      (bind _returnvalue (`GameplayStatics.LoadGameFromSlot` "BestScore"))
      (bind _asbp_save_game (cast `/Game/Blueprints/BP_SaveGame` _returnvalue))
      (bind _output_get_2 (set `self.SaveGameInstance_Ref` _asbp_save_game))
      (`/Engine/EditorBlueprintResources/StandardMacros.CompareInt` (`/Game/Blueprints/BP_SaveGame.BestScore` _output_get_2) (`self.Score`)
        (:`==`
          _)
        (:`<`
          _))
      (bind _output_get_3 (set `/Game/Blueprints/BP_SaveGame.BestScore` (`self.Score`) _savegameinstance_ref))
      (`TextBlock.SetText` (`/Game/Blueprints/WG_GameHUD.BestScoreText` (`self.HUD_Ref`)) (`KismetTextLibrary.Conv_IntToText` _output_get_3 false false))
      (`GameplayStatics.SaveGameToSlot` _savegameinstance_ref "BestScore"))))

(event `CheckSaveGameSlot`
  (bind _returnvalue (`GameplayStatics.DoesSaveGameExist` "BestScore"))
  (if _returnvalue
    (bind _returnvalue_2 (`GameplayStatics.LoadGameFromSlot` "BestScore"))
    (bind _asbp_save_game (cast `/Game/Blueprints/BP_SaveGame` _returnvalue_2))
    (bind _output_get (set `self.SaveGameInstance_Ref` _asbp_save_game))
    (`TextBlock.SetText` (`/Game/Blueprints/WG_GameHUD.BestScoreText` (`self.HUD_Ref`)) (`KismetTextLibrary.Conv_IntToText` (`/Game/Blueprints/BP_SaveGame.BestScore` _output_get) false false))
    (else
      (bind _returnvalue_3 (`GameplayStatics.CreateSaveGameObject` "/Game/Blueprints/BP_SaveGame.BP_SaveGame_C"))
      (bind _asbp_save_game_2 (cast `/Game/Blueprints/BP_SaveGame` _returnvalue_3))
      (bind _output_get_2 (set `self.SaveGameInstance_Ref` _asbp_save_game_2))
      (bind _output_get_3 (set `/Game/Blueprints/BP_SaveGame.BestScore` 0 _output_get_2))
      (`TextBlock.SetText` (`/Game/Blueprints/WG_GameHUD.BestScoreText` (`self.HUD_Ref`)) (`KismetTextLibrary.Conv_IntToText` _output_get_3 false false))
      (`GameplayStatics.SaveGameToSlot` _output_get_2 "BestScore"))))

(fn `UserConstructionScript`)